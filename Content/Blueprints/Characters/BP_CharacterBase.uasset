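; Base character Blueprint that gives combatants shared health, melee attack and hit-reaction logic.
; CallAttackBoxTrace box-traces for another BP_CharacterBase, triggers its reactions, disables input, applies damage and messages BPI_Player targets for death checking.
; Reactions spawn particles and a floating damage number projected to screen, playing an override animation only if the hit is non-lethal.
; AnyDamage lowers clamped health; DisableBT is an empty stub.
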(event `self.ReceiveBeginPlay`
  ;[0 0.15 0.1008 0.5] Set Health Equal To Max Health
  (`self.SetEssentialVariables`)
  (`self.SetHealthToMaxHealth`)
  (set `self.IsAlive` true))

(event `/Game/Interfaces/BPI_AttackTrace.CallAttackBoxTrace`
  ;[0 0.15 0.03487 0.5] Attack Tracing
  (`self.GetHit` (`self.Attack Damage`)))

(event `self.ReceiveAnyDamage`
  (params (Damage :type "Float (single-precision)") (DamageType :type "DamageType Object Reference") (InstigatedBy :type "Controller Object Reference") (DamageCauser :type "Actor Object Reference"))
  ;[0.15 0.003159 0 0.5] Take Damage
  (`self.DecrementHealth` Damage))

(fn `AttackOpponentAnimation`
  (`PaperZDAnimInstance.K2_PlayAnimationOverride` (`PaperZDAnimationComponent.AnimInstance` (`self.Animation Component`)) (`self.AttackAnimSequence`) (`self.AnimOverrideSlot`) 1.0 0.0))

(fn `BoxTraceOpponents`
  (returns (OutHit :type "HitResult Structure"))
  (bind _outhit (`KismetSystemLibrary.BoxTraceSingleForObjects` (`SceneComponent.K2_GetComponentLocation` (`self.Box Trace Start`)) (`SceneComponent.K2_GetComponentLocation` (`self.Box Trace End`)) (`self.TraceExtent`) (`self.BoxRotation`) (`self.TraceObjectTypes`)))
  (return _outhit))

(fn `CheckForRedhoodDeath`
  (params (DamageActor :type "Object Object Reference"))
  (if (`KismetSystemLibrary.DoesImplementInterface` DamageActor "/Game/Interfaces/BPI_Player.BPI_Player_C")
    (message `/Game/Interfaces/BPI_Player.PlayerDeath` DamageActor)))

(fn `CreateDamageNumber`
  (params (Number :type "Float (double-precision)") (Location :type "Vector Structure"))
  (locals (NumberWidget :type "/Game/UI/WBP_DamageNumber Object Reference"))
  (bind (_location_x _location_y _location_z) (`KismetMathLibrary.BreakVector` (`local.Location`)))
  (bind _numberwidget (`local.NumberWidget`))
  (`self.PlayerController`
    (:`then`
      (`|ExecutionSequence`
        (:`then_0`
          ;[0.003523 0.000305 0.15 0.5] Create Damage Number Widget
          (bind _returnvalue (`|CreateWidget` "/Game/UI/WBP_DamageNumber.WBP_DamageNumber_C" (`self.PlayerController`)))
          (bind _output_get (set `local.NumberWidget` _returnvalue))
          (`UserWidget.AddToViewport` _output_get 0))
        (:`then_1`
          ;[0.000307 0.1345 0.15 0.5] Set Damage Number Attributes and Value
          (`/Game/UI/WBP_DamageNumber.SetNumber` (`local.NumberWidget`) (`local.Number`) (`self.DamageNumber_sRGB`)))
        (:`then_2`
          ;[0.15 0.09671 0 0.5] Set Damage Number Pos in Viewport
          (`UserWidget.SetPositionInViewport` (`local.NumberWidget`) (`GameplayStatics.ProjectWorldToScreen` (`self.PlayerController`) (`KismetMathLibrary.MakeVector` _location_x _location_y (+ _location_z 75.0))) true))
        (:`then_3`
          ;[0 0.1285 0.15 0.5] Play Damage Number Animation
          (`UserWidget.PlayAnimation` _numberwidget (`/Game/UI/WBP_DamageNumber.FloatingAnim` _numberwidget) 0.0 1 "Forward" 1.0 false))))
    (:`else`)))

(fn `DecrementHealth`
  (params (Damage :type "Float (double-precision)"))
  (set `self.Health` (`KismetMathLibrary.FClamp` (- (`self.Health`) Damage) 0.0 (`self.MaxHealth`))))

(fn `DisableBT`)

(fn `GetHit`
  (params (`Take Damage` :type "Float (double-precision)"))
  ;[0.15 0.1413 0 0.5] Box Trace For Opponent
  (bind _outhit (`self.BoxTraceOpponents`))
  ;[0 0.15 0.1223 0.5] Play Hit React On Opponent
  (bind _asbp_character_base (cast `/Game/Blueprints/Characters/BP_CharacterBase` (`.HitActor` (`GameplayStatics.BreakHitResult` _outhit))))
  (`self.PlayGetHitReactions` _asbp_character_base `Take Damage`)
  (`self.SetInputEnabled` _asbp_character_base false)
  (`GameplayStatics.ApplyDamage` _asbp_character_base `Take Damage`)
  (`self.CheckForRedhoodDeath` _asbp_character_base))

(fn `GetHitEffects`
  (`NiagaraFunctionLibrary.SpawnSystemAtLocation` (`self.HitParticles`) (`self.K2_GetActorLocation`)))

(fn `PlayGetHitReactions`
  (params (`In Damage` :type "Float (double-precision)"))
  (`self.PlayHitReactAnimation` `In Damage`)
  (`self.GetHitEffects`)
  (`self.CreateDamageNumber` `In Damage` (`self.K2_GetActorLocation`)))

(fn `PlayHitReactAnimation`
  (params (Damage :type "Float (double-precision)"))
  (if (> (- (`self.Health`) (`local.Damage`)) 0.0)
    (`PaperZDAnimInstance.K2_PlayAnimationOverride` (`PaperZDAnimationComponent.AnimInstance` (`self.Animation Component`)) (`self.HitReactSequence`) (`self.AnimOverrideSlot`) 1.0 0.0)))

(fn `SetEssentialVariables`
  (set `self.PlayerController` (`GameplayStatics.GetPlayerController` 0)))

(fn `SetHealthToMaxHealth`
  (set `self.Health` (`self.MaxHealth`)))

(fn `SetInputEnabled`
  (params (Enabled :type Boolean))
  (`self.PlayerController`
    (:`then`
      (if Enabled
        (`self.EnableInput` (`self.PlayerController`))
        (else
          (`self.DisableInput` (`self.PlayerController`)))))
    (:`else`)))

(fn `UserConstructionScript`)