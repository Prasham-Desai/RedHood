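; BP_EnemyBase is a base enemy character Blueprint that links combat targeting, attack animation and turning to AI behavior.
; SetCombatTarget writes the given target into the AI controller's Blackboard under a configurable key name for the behavior tree.
; PlayAttackAnim forwards to AttackOpponentAnimation, and ChangeDirection rotates the actor by combining its current rotation with a stored rotator offset.
; BeginPlay only calls the parent implementation.
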(event `self.ReceiveBeginPlay`
  (`parent.ReceiveBeginPlay`))

(event `/Game/Interfaces/BPI_Enemy.SetCombatTarget`
  (params (`Combat Target` :type "Actor Object Reference"))
  ;[0 0.15 0.1198 0.5] Set combat target for BT
  (`BlackboardComponent.SetValueAsObject` (`AIBlueprintHelperLibrary.GetBlackboard` (`self.GetController`)) (`self.CombatTargetBBKeyName`) `Combat Target`))

(event `/Game/Interfaces/BPI_Enemy.PlayAttackAnim`
  ;[0.15 0.03526 0 0.5] Play Attack Animation
  (`self.AttackOpponentAnimation`))

(fn `ChangeDirection`
  (`self.K2_SetActorRotation` (`KismetMathLibrary.ComposeRotators` (`self.K2_GetActorRotation`) (`self.ChangeDirRotator`))))

(fn `UserConstructionScript`)