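; BP_Skeleton is an enemy skeleton character that patrols by walking constantly in the direction it faces.
; On BeginPlay, StartPatrolling calls ChangeDirection once, then starts a looping timer by function name, using variables for the name and interval.
; Every Tick, MoveSkeleton feeds the actor's forward vector into AddMovementInput at full scale.
; The body of ChangeDirection is not defined in these graphs.
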(event `self.ReceiveBeginPlay`
  ;[5e-06 0.1498 0.15 0.5] Enemy Patrol
  (`self.StartPatrolling`))

(event `self.ReceiveTick`
  (params (DeltaSeconds :type "Float (single-precision)"))
  ;[0 0.15 0.1408 0.5] Move Skeleton
  (`self.MoveSkeleton`))

(fn `MoveSkeleton`
  (`self.AddMovementInput` (`self.GetActorForwardVector`)))

(fn `StartPatrolling`
  (`self.ChangeDirection`)
  (`KismetSystemLibrary.K2_SetTimer` null (`self.ChangeDirFunctionName`) (`self.ChangeDirInSeconds`) true))

(fn `UserConstructionScript`)